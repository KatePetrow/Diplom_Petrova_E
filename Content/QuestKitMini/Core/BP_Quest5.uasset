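; BP_Quest5 is a three-stage timing puzzle where the player clicks the active button while its moving line is inside a hidden target zone.
; While the player view is active, Tick bounces the current line between limits and turns it green near its random Password position.
; A correct click advances and a miss steps back one, with timed button color feedback; clearing the third calls OnWin.
; View changes before a win reset progress and reroll the targets.
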(event `self.ReceiveTick`
  (params (DeltaSeconds :type "Float (single-precision)"))
  ;[1 1 1] Move
  (if (`self.isWin`)
    _
    (elif (`self.Enable`)
      (`self.Move` (`self.Index`)))))

(event `self.ReceiveBeginPlay`
  ;[1 1 1] BeginPlay
  (`parent.ReceiveBeginPlay`)
  (`self.GeneratePass`)
  (add `PrimitiveComponent.OnClicked` (`self.2`) (delegate `OnClick`))
  (add `PrimitiveComponent.OnClicked` (`self.1`) (delegate `OnClick`))
  (add `PrimitiveComponent.OnClicked` (`self.0`) (delegate `OnClick`)))

(event `OnClick`
  (params (TouchedComponent :type "PrimitiveComponent Object Reference") (ButtonPressed :type "Key Structure" :default "None"))
  ;[1 1 1] BeginPlay
  (if (not (`self.isWin`))
    (`self.ButtonClick` (`KismetStringLibrary.Conv_StringToInt` (`KismetSystemLibrary.GetObjectName` TouchedComponent)))))

(event `ButtonAction`
  (params (isCorrect :type Boolean))
  ;[1 1 1] Button click
  (set `self.EnableButtons` false)
  (bind _output_get (set `self.IndexButton` (`self.Index`)))
  (`self.SetButtonStyle` _output_get (select `bool` isCorrect :`false` 3 :`true` 2 :!type "Byte"))
  (bind _returnvalue (`KismetSystemLibrary.K2_SetTimerDelegate` (delegate `StyleTick`) (`self.BlinkButtonDilay`)))
  (set `self.TimerButtonStyle` _returnvalue))

(event `StyleTick`
  ;[1 1 1] Button click
  (`self.SetButtonStyle` (`self.IndexButton`))
  (`self.SetButtonStyle` (`self.Index`) 1)
  (set `self.EnableButtons` true))

(fn `ButtonClick`
  (params (Index :type Integer))
  (bind _passcorrect (`self.PassCorrect`))
  (bind _index (`self.Index`))
  (bind _index_2 (`self.Index`))
  (if (and (== Index (`KismetMathLibrary.Conv_ByteToInt` (`self.Index`))) (`self.EnableButtons`))
    (`self.SetLineStyle` (`self.Index`))
    (`self.ButtonAction` _passcorrect)
    (if _passcorrect
      (if (== _index_2 2)
        (`self.onWin` self)
        (set `self.EnableButtons` false)
        (set `self.isWin` true)
        (`self.SetButtonStyle` (`self.Index`))
        (`KismetSystemLibrary.K2_ClearAndInvalidateTimerHandle` (`self.TimerButtonStyle`))
        (else
          (set `self.Index` (+ _index_2 1))))
      (else
        (set `self.Index` (- _index (select `bool` (== _index 0) :`false` 1 :!type "Byte")))))))

(fn `GeneratePass`
  (bind _password (`self.Password`))
  (`KismetArrayLibrary.Array_Clear` _password)
  (for _ (range 3)
    (`KismetArrayLibrary.Array_Add` _password (`KismetMathLibrary.RandomFloatInRange` (`self.MinPosition`) (`self.MaxPosition`)))))

(fn `Move`
  (params (Index :type Byte))
  (bind _returnvalue (`KismetMathLibrary.Conv_ByteToInt` Index))
  (bind _output (`|GetArrayItem` (`self.Direction`) _returnvalue))
  (bind _output_2 (`|GetArrayItem` (`self.Password`) (`KismetMathLibrary.Conv_ByteToInt` Index)))
  (bind _returnvalue_2 (select `byte` Index :`0` (`self.SM_Line1`) :`1` (`self.SM_Line2`) :`2` (`self.SM_Line3`) :!type "SceneComponent Object Reference"))
  (bind (_relativelocation_x _relativelocation_y _relativelocation_z) (`KismetMathLibrary.BreakVector` (`SceneComponent.RelativeLocation` _returnvalue_2)))
  (bind _output_get (set `self.PassCorrect` (and (> _relativelocation_y (- _output_2 (`self.ZoneSize`))) (< _relativelocation_y (+ _output_2 (`self.ZoneSize`))))))
  (`self.SetLineStyle` Index (select `bool` _output_get :`true` 2 :!type "Byte"))
  (if (and (< _relativelocation_y (`self.MinPosition`)) (== _output -1.0))
    (`KismetArrayLibrary.Array_Set` (`self.Direction`) _returnvalue 1.0))
  (if (and (> _relativelocation_y (`self.MaxPosition`)) (== _output 1.0))
    (`KismetArrayLibrary.Array_Set` (`self.Direction`) _returnvalue -1.0))
  (`SceneComponent.K2_SetRelativeLocation` _returnvalue_2 (`KismetMathLibrary.MakeVector` _relativelocation_x (+ _relativelocation_y (* (`GameplayStatics.GetWorldDeltaSeconds`) _output (`self.Speed`))) _relativelocation_z) false false))

(fn `PlayerView`
  (params (isIn :type Boolean))
  (`parent.PlayerView` false)
  (if (not (`self.isWin`))
    (bind _output_get (set `self.Enable` isIn))
    (`self.Reset`)
    (if _output_get
      (`self.SetLineStyle` 0)
      (`self.SetButtonStyle` 0 1))))

(fn `Reset`
  (set `self.Index` 0)
  (`KismetSystemLibrary.K2_ClearAndInvalidateTimerHandle` (`self.TimerButtonStyle`))
  (set `self.EnableButtons` true)
  (`self.GeneratePass`)
  (for (_ _array_index) (`self.Password`)
    (bind _returnvalue (`KismetMathLibrary.Conv_IntToByte` _array_index))
    (`self.SetButtonStyle` _returnvalue)
    (`self.SetLineStyle` _returnvalue)))

(fn `SetButtonStyle`
  (params (Index :type Byte) (Style :type Byte))
  (`PrimitiveComponent.SetMaterial` (select `byte` Index :`0` (`self.0`) :`1` (`self.1`) :`2` (`self.2`) :!type "PrimitiveComponent Object Reference") 0 (select `byte` Style :`0` "/Game/QuestKitMini/Materials/MI_BaseC.MI_BaseC" :`1` "/Game/QuestKitMini/Materials/M_BaseEmissive.M_BaseEmissive" :`2` "/Game/QuestKitMini/Materials/MI_GreenEmissive.MI_GreenEmissive" :`3` "/Game/QuestKitMini/Materials/MI_RedEmissive.MI_RedEmissive" :!type "MaterialInterface Object Reference")))

(fn `SetLineStyle`
  (params (Index :type Byte) (Style :type Byte))
  (`PrimitiveComponent.SetMaterial` (select `byte` Index :`0` (`self.SM_Line1`) :`1` (`self.SM_Line2`) :`2` (`self.SM_Line3`) :!type "PrimitiveComponent Object Reference") 0 (select `byte` Style :`0` "/Game/QuestKitMini/Materials/M_BaseEmissive_InstLow.M_BaseEmissive_InstLow" :`1` "/Game/QuestKitMini/Materials/M_BaseEmissive.M_BaseEmissive" :`2` "/Game/QuestKitMini/Materials/MI_GreenEmissive.MI_GreenEmissive" :!type "MaterialInterface Object Reference")))

(fn `UserConstructionScript`)