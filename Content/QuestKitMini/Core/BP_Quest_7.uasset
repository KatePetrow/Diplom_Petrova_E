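; BP_Quest_7 is a code-entry puzzle where numbered, clickable meshes must be pressed in the order of a displayed code.
; The construction script builds a row of labelled buttons and lights, tagging each button with its index.
; CodeGeneration shuffles the indices and displays them; correct clicks light lamps, while mistakes reset all progress lights.
; Completing the first round generates a new code, and the second consecutive success calls OnWin.
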(event `self.ReceiveBeginPlay`
  (`parent.ReceiveBeginPlay`)
  (`self.CodeGeneration`))

(fn `ButtonClick`
  (params (TouchedComponent :type "PrimitiveComponent Object Reference") (ButtonPressed :type "Key Structure" :default "None"))
  (bind _returnvalue (`KismetStringLibrary.Conv_StringToInt` (`KismetStringLibrary.Conv_NameToString` (`|GetArrayItem` (`ActorComponent.ComponentTags` TouchedComponent)))))
  (if (== (`|GetArrayItem` (`self.Code`) (`self.ClickIndex`)) _returnvalue)
    (`self.LightSwitch` _returnvalue)
    (`/Engine/EditorBlueprintResources/StandardMacros.IncrementInt` (`self.ClickIndex`)
      (:`  `
        (`self.CheckWin`)))
    (else
      (`self.OffAll`)
      (set `self.ClickIndex` 0)
      (`self.ResetWin`))))

(fn `CheckWin`
  (locals (isWin :type Boolean))
  (set `local.isWin` true)
  (for _array_element (`self.LightsStatus`)
    (if (not _array_element)
      (set `local.isWin` false)))
  (if (`local.isWin`)
    (bind _result (`/Engine/EditorBlueprintResources/StandardMacros.IncrementInt` (`self.Win`))
      (:`  `
        (if (== _result 2)
          (`self.onWin` self)
          (`PrimitiveComponent.SetMaterial` (`self.LightWin2`) 0 (`self.MaterialWin`))
          (else
            (`PrimitiveComponent.SetMaterial` (`self.LightWin1`) 0 (`self.MaterialWin`))
            (`self.OffAll`)
            (`self.CodeGeneration`)))))))

(fn `CodeGeneration`
  (locals (Digital :type "Array of Integer") (RandomIndex :type Integer))
  (bind _digital (`local.Digital`))
  (`KismetArrayLibrary.Array_Clear` (`self.Code`))
  (for _index (range (+ (`self.CodeLen`) 1))
    (`KismetArrayLibrary.Array_Add` (`local.Digital`) _index))
  (for _ (range (+ (`self.CodeLen`) 1))
    (bind _output_get (set `local.RandomIndex` (`KismetMathLibrary.RandomInteger` (`KismetArrayLibrary.Array_Length` _digital))))
    (`KismetArrayLibrary.Array_Add` (`self.Code`) (`|GetArrayItem` _digital _output_get))
    (`KismetArrayLibrary.Array_Remove` _digital _output_get))
  (`self.DisplayCode`))

(fn `DisplayCode`
  (set `self.CodeStr` "")
  (for _array_element (`self.Code`)
    (set `self.CodeStr` (`KismetStringLibrary.Concat_StrStr` (`self.CodeStr`) (`KismetStringLibrary.Conv_IntToString` _array_element) " ")))
  (`TextRenderComponent.K2_SetText` (`self.TextRender`) (`KismetTextLibrary.Conv_StringToText` (`self.CodeStr`))))

(fn `LightSwitch`
  (params (id :type Integer))
  (locals (NewStatus :type Boolean))
  (bind _lightsstatus (`self.LightsStatus`))
  (bind _output_get (set `local.NewStatus` (not (`|GetArrayItem` _lightsstatus id))))
  (`KismetArrayLibrary.Array_Set` _lightsstatus id _output_get)
  (`PrimitiveComponent.SetMaterial` (`|GetArrayItem` (`self.Lights`) id) 0 (select `bool` (`local.NewStatus`) :`false` (`self.MaterialOff`) :`true` (`self.MaterialOn`))))

(fn `OffAll`
  (bind _lightsstatus (`self.LightsStatus`))
  (for (_ _array_index) _lightsstatus
    (`KismetArrayLibrary.Array_Set` _lightsstatus _array_index)
    (`PrimitiveComponent.SetMaterial` (`|GetArrayItem` (`self.Lights`) _array_index) 0 (`self.MaterialOff`))
    (set `self.ClickIndex` 0)))

(fn `ResetWin`
  (set `self.Win` 0)
  (`PrimitiveComponent.SetMaterial` (`self.LightWin1`) 0 (`self.MaterialOff`)))

(fn `UserConstructionScript`
  (bind (_startposition_x _startposition_y _startposition_z) (`KismetMathLibrary.BreakVector` (`self.StartPosition`)))
  (for _index (range (+ (`self.CodeLen`) 1))
    (bind _returnvalue (+ _startposition_y (`KismetMathLibrary.Conv_IntToDouble` (* _index -8))))
    (bind _returnvalue_2 (`AddComponent|NODE_AddTextRenderComponent-0` :`RelativeTransform` (`KismetMathLibrary.MakeTransform` (`KismetMathLibrary.MakeVector` 4.2 _returnvalue (+ _startposition_z -3.0)) (struct) (0.2 0.2 0.2))))
    (bind _returnvalue_3 (`KismetStringLibrary.Conv_IntToString` _index))
    (`TextRenderComponent.K2_SetText` _returnvalue_2 (`KismetTextLibrary.Conv_StringToText` _returnvalue_3))
    (bind _returnvalue_4 (`AddComponent|NODE_AddStaticMeshComponent-0` :`RelativeTransform` (`KismetMathLibrary.MakeTransform` (`KismetMathLibrary.MakeVector` (+ _startposition_x -2.0) _returnvalue _startposition_z))))
    (`SceneComponent.K2_AttachToComponent` _returnvalue_4 (`self.DefaultSceneRoot`) "None" "KeepRelative" "KeepRelative" "KeepRelative" true)
    (set `ActorComponent.ComponentTags` (`|MakeArray` (`KismetStringLibrary.Conv_StringToName` _returnvalue_3)) _returnvalue_4)
    (add `PrimitiveComponent.OnClicked` _returnvalue_4 (`|CreateDelegate` :!event `ButtonClick`))
    (bind _returnvalue_5 (`AddComponent|NODE_AddStaticMeshComponent-2` :`RelativeTransform` (`KismetMathLibrary.MakeTransform` (`KismetMathLibrary.MakeVector` _startposition_x _returnvalue (+ _startposition_z 10.0)))))
    (`SceneComponent.K2_AttachToComponent` _returnvalue_5 (`self.DefaultSceneRoot`) "None" "KeepRelative" "KeepRelative" "KeepRelative" true)
    (`KismetArrayLibrary.Array_Add` (`self.Lights`) _returnvalue_5)
    (`KismetArrayLibrary.Array_Add` (`self.LightsStatus`))))