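; Base interactive panel actor that the player enters and leaves through the BIInteraction event.
; SetView toggles IsInteractive, blending the camera between the controlled pawn and the panel.
; While active, it shows the cursor, enables click events and Game-and-UI input, and locks character movement and look; leaving switches to game-only input and walking.
; An empty PlayerView function receives the new state, apparently as an override hook for child panels.
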(event `/Game/QuestKitMini/Core/BI_Interact.BI_Interaction`
  (`self.Set View`))

(fn `PlayerView`
  (params (isIn :type Boolean)))

(fn `Set View`
  (bind _returnvalue (`GameplayStatics.GetPlayerController` 0))
  (bind _returnvalue_2 (`GameplayStatics.GetPlayerController` 0))
  (bind _pawn (`self.Pawn`))
  (set `self.Pawn` (`Controller.K2_GetPawn` _returnvalue))
  (`PlayerController.SetViewTargetWithBlend` _returnvalue (select `bool` (`self.isInteractive`) :`false` self :`true` (`self.Pawn`) :!type "Actor Object Reference") 1.0 "VTBlend_Linear" 0.0 false)
  (bind _output_get (set `self.isInteractive` (not (`self.isInteractive`))))
  (set `PlayerController.bShowMouseCursor` _output_get _returnvalue)
  (if _output_get
    (`WidgetBlueprintLibrary.SetInputMode_GameAndUIEx` _returnvalue null "DoNotLock" false)
    (set `PlayerController.bEnableClickEvents` true _returnvalue)
    (`self.PlayerView` true)
    (bind _ascharacter (cast `Character` _pawn))
    (bind _charactermovement (`Character.CharacterMovement` _ascharacter))
    (`CharacterMovementComponent.DisableMovement` _charactermovement)
    (set `CharacterMovementComponent.bOrientRotationToMovement` false _charactermovement)
    (`Controller.SetIgnoreLookInput` _returnvalue_2 true)
    (else
      (`WidgetBlueprintLibrary.SetInputMode_GameOnly` _returnvalue)
      (set `PlayerController.bEnableClickEvents` false _returnvalue)
      (`self.PlayerView` false)
      (bind _ascharacter_2 (cast `Character` _pawn))
      (bind _charactermovement_2 (`Character.CharacterMovement` _ascharacter_2))
      (`CharacterMovementComponent.SetMovementMode` _charactermovement_2 "MOVE_Walking" 0)
      (set `CharacterMovementComponent.bOrientRotationToMovement` true _charactermovement_2)
      (`Controller.SetIgnoreLookInput` _returnvalue_2 false))))

(fn `UserConstructionScript`)