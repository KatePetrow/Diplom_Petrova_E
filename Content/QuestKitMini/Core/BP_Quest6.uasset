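; Card-swipe quest puzzle in QuestKitMini, won by dragging a card through a reader at the right speed.
; Clicking the card makes it follow mouse Y on Tick, timing the swipe from when it leaves the top dead zone to the bottom.
; A time within tolerance fires OnWin and lights green; otherwise text shows Fast or Slow with a brief red LED.
; The PlayerView override toggles and resets the card until won.
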(event `self.ReceiveTick`
  (params (DeltaSeconds :type "Float (single-precision)"))
  (bind _card (`self.Card`))
  (bind _needtimeallowzone (`self.NeedTimeAllowZone`))
  (bind _needtime (`self.NeedTime`))
  (bind _returnvalue (- (`KismetSystemLibrary.GetGameTimeInSeconds`) (`self.Time`)))
  (bind (_relativelocation_x _relativelocation_y) (`KismetMathLibrary.BreakVector` (`SceneComponent.RelativeLocation` _card)))
  (bind _returnvalue_2 (< (- _returnvalue _needtimeallowzone) _needtime))
  (bind _returnvalue_3 (`KismetMathLibrary.FClamp` (* -1 (/ (- (`.LocationY` (`WidgetLayoutLibrary.GetMousePositionScaledByDPI` (`GameplayStatics.GetPlayerController` 0))) (`self.StartMouseY`)) 15.0)) (`self.EndZ`) (`self.StartZ`)))
  ;[1 1 1] Card move
  (if (`self.StartMove`)
    (if (> (+ _returnvalue_3 0.1) (`self.StartZ`))
      (set `self.Time` (`KismetSystemLibrary.GetGameTimeInSeconds`)))
    (if (== _returnvalue_3 (`self.EndZ`))
      (set `self.StartMove` false)
      ;[1 1 1] Card move end
      (`SceneComponent.K2_SetRelativeLocation` _card (`KismetMathLibrary.MakeVector` _relativelocation_x _relativelocation_y (`self.StartZ`)) false false)
      (if (`self.Debug`)
        (`KismetSystemLibrary.PrintString` (`KismetStringLibrary.Conv_DoubleToString` _returnvalue) true true (struct :`R` 1.0 :`G` 0.119454 :`A` 1.0)))
      (if (and (> (+ _needtimeallowzone _returnvalue) _needtime) _returnvalue_2)
        ;[1 1 1] Valid, win
        (`self.onWin` self)
        (`self.SetStyle` 2)
        (`TextRenderComponent.K2_SetText` (`self.TextRender`) "")
        (`SceneComponent.SetVisibility` (`self.Card`) false false)
        (`KismetSystemLibrary.K2_ClearAndInvalidateTimerHandle` (`self.LedTimer`))
        (set `self.isWin` true)
        (set `self.EnableClick` false)
        (else
          ;[1 1 1] No valid
          (set `self.EnableClick` true)
          (`TextRenderComponent.K2_SetText` (`self.TextRender`) (`KismetTextLibrary.Conv_StringToText` (select `bool` _returnvalue_2 :`false` "Slow" :`true` "Fast")))
          (`self.SetStyle` 1)
          (bind _returnvalue_4 (`KismetSystemLibrary.K2_SetTimerDelegate` (delegate `LedOff`) 1.0))
          (set `self.LedTimer` _returnvalue_4)))
      (else
        (`SceneComponent.K2_SetRelativeLocation` _card (`KismetMathLibrary.MakeVector` _relativelocation_x _relativelocation_y _returnvalue_3) false false)))))

(event `LedOff`
  ;[1 1 1] No valid
  (`self.SetStyle` 0))

(event `self.Card.OnClicked`
  (params (TouchedComponent :type "PrimitiveComponent Object Reference") (ButtonPressed :type "Key Structure"))
  ;[1 1 1] Card click
  (if (`self.EnableClick`)
    (set `self.EnableClick` false)
    (set `self.StartMove` true)
    (set `self.StartMouseY` (`.LocationY` (`WidgetLayoutLibrary.GetMousePositionScaledByDPI` (`GameplayStatics.GetPlayerController` 0))))))

(fn `PlayerView`
  (params (isIn :type Boolean))
  (bind _card (`self.Card`))
  (bind (_relativelocation_x _relativelocation_y) (`KismetMathLibrary.BreakVector` (`SceneComponent.RelativeLocation` _card)))
  (`parent.PlayerView` isIn)
  (if (not (`self.isWin`))
    (`SceneComponent.SetVisibility` (`self.Card`) isIn false)
    (set `self.EnableClick` isIn)
    (set `self.StartMove` false)
    (`SceneComponent.K2_SetRelativeLocation` _card (`KismetMathLibrary.MakeVector` _relativelocation_x _relativelocation_y (`self.StartZ`)) false false)))

(fn `SetStyle`
  (params (Byte :type Byte))
  (bind _reader (`self.Reader`))
  (`PrimitiveComponent.SetMaterial` _reader 2 (select `byte` Byte :`0` "/Game/QuestKitMini/Materials/MI_BaseC.MI_BaseC" :`1` "/Game/QuestKitMini/Materials/MI_BaseC.MI_BaseC" :`2` "/Game/QuestKitMini/Materials/MI_EmissiveBase_G.MI_EmissiveBase_G" :!type "MaterialInterface Object Reference"))
  (`PrimitiveComponent.SetMaterial` _reader 3 (select `byte` Byte :`0` "/Game/QuestKitMini/Materials/MI_BaseC.MI_BaseC" :`1` "/Game/QuestKitMini/Materials/MI_EmissiveBase_R.MI_EmissiveBase_R" :`2` "/Game/QuestKitMini/Materials/MI_BaseC.MI_BaseC" :!type "MaterialInterface Object Reference")))

(fn `UserConstructionScript`)