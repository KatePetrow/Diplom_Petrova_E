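; BP_Quest_1 is a quest actor where a button click starts a timed progress task that ends in a win.
; While enabled, processing and interactive, Tick advances progress by Speed, then calls OnWin, disables itself and shows the win text when full.
; Losing interactivity mid-process resets progress and status.
; A dynamic material instance created in the construction script drives the progress cube's display through a scalar parameter.
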(event `self.ReceiveTick`
  (params (DeltaSeconds :type "Float (single-precision)"))
  (if (`self.Enable`)
    (if (`self.Processing`)
      (if (`self.isInteractive`)
        (bind _output_get (set `self.Progress` (`KismetMathLibrary.FClamp` (+ (* (`self.Speed`) DeltaSeconds) (`self.Progress`)))))
        (`MaterialInstanceDynamic.SetScalarParameterValue` (`self.ProgressMat`) "Progress" _output_get)
        (if (== _output_get 1.0)
          (`self.onWin` self)
          (set `self.Enable` false)
          (`TextRenderComponent.K2_SetText` (`self.TextRender`) (`self.WinText`)))
        (else
          (`self.Reset`))))))

(event `self.Button.OnClicked`
  (params (TouchedComponent :type "PrimitiveComponent Object Reference") (ButtonPressed :type "Key Structure"))
  (set `self.Processing` true)
  (`self.UpdateStatus`))

(fn `Reset`
  (`MaterialInstanceDynamic.SetScalarParameterValue` (`self.ProgressMat`) "Progress" 0.0)
  (set `self.Processing` false)
  (set `self.Progress` 0.0)
  (`self.UpdateStatus`))

(fn `UpdateStatus`
  (`TextRenderComponent.K2_SetText` (`self.TextRender`) (select `bool` (`self.Processing`) :`false` "Ready" :`true` "Processing...")))

(fn `UserConstructionScript`
  (bind _returnvalue (`KismetMaterialLibrary.CreateDynamicMaterialInstance` "/Game/QuestKitMini/Materials/MI_Progress.MI_Progress"))
  (set `self.ProgressMat` _returnvalue)
  (`PrimitiveComponent.SetMaterial` (`self.CubeProgress`) 0 _returnvalue))