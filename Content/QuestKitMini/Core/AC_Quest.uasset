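; Quest component that tracks quest panels and provides player interaction in the QuestKitMini kit.
; One second after BeginPlay it gathers all BP_PanelBase actors as quests and binds their OnWin events to Win, which only prints optional debug text.
; Interaction line-traces forward from the player camera on Visibility, sends the BI_Interact message to a hit actor implementing that interface, and returns whether it did.
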(event `self.ReceiveBeginPlay`
  (`KismetSystemLibrary.Delay` 1.0)
  (bind _outactors (`GameplayStatics.GetAllActorsOfClass` "/Game/QuestKitMini/Core/BP_PanelBase.BP_PanelBase_C"))
  (bind _output_get (set `self.Quests` _outactors))
  (for _array_element _output_get
    (add `/Game/QuestKitMini/Core/BP_PanelBase.onWin` _array_element (delegate `Win`))
    ;[1 0 0.6908] Debug quest list
    (if (`self.Debug`)
      (`KismetSystemLibrary.PrintString` (`KismetStringLibrary.Concat_StrStr` "Quest detect: " (`KismetTextLibrary.Conv_TextToString` (`/Game/QuestKitMini/Core/BP_PanelBase.Name` _array_element))) true true (struct :`R` 0.851748 :`B` 1.0 :`A` 1.0)))))

(event `Win`
  (params (QuestRef :type "/Game/QuestKitMini/Core/BP_PanelBase Object Reference"))
  ;[1 0 0.8167] Debug win
  (if (`self.Debug`)
    (`KismetSystemLibrary.PrintString` (`KismetStringLibrary.Concat_StrStr` "Win: \" " (`KismetTextLibrary.Conv_TextToString` (`/Game/QuestKitMini/Core/BP_PanelBase.Name` QuestRef)) "\"") true true (struct :`R` 0.854993 :`B` 1.0 :`A` 1.0))))

(fn `Interaction`
  (returns (isOk :type Boolean))
  (bind _rootcomponent (`Actor.RootComponent` (`GameplayStatics.GetPlayerCameraManager` 0)))
  (bind _returnvalue (`SceneComponent.K2_GetComponentLocation` _rootcomponent))
  ;[1 0 0.02628] Interaction
  (bind _outhit (`KismetSystemLibrary.LineTraceSingle` _returnvalue (+ (* (`SceneComponent.GetForwardVector` _rootcomponent) 1000.0) _returnvalue) "TraceTypeQuery1"))
  (if (`GameplayStatics.BreakHitResult` _outhit)
    (if (`KismetSystemLibrary.DoesImplementInterface` (`.HitActor` (`GameplayStatics.BreakHitResult` _outhit)) "/Game/QuestKitMini/Core/BI_Interact.BI_Interact_C")
      (message `/Game/QuestKitMini/Core/BI_Interact.BI_Interaction` (`.HitActor` (`GameplayStatics.BreakHitResult` _outhit)))
      (return true)
      (else
        _)))
  (return false))