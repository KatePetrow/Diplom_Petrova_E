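; BP_Quest_9 is a combination-dial quest puzzle where horizontal mouse dragging spins a clicked mesh toward random target angles.
; CheckPosition lights an indicator green while yaw sits within the current target's zone.
; Each drag-direction reversal triggers CheckPass, which either advances the progress lights or resets progress and regenerates targets, flashing red if progress was lost.
; Completing the sequence calls the win handler and SetView, then disables input handling.
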(event `self.ReceiveBeginPlay`
  (`parent.ReceiveBeginPlay`)
  (`self.GeneratePass`))

(event `self.ReceiveTick`
  (params (DeltaSeconds :type "Float (single-precision)"))
  (bind _returnvalue (`GameplayStatics.GetPlayerController` 0))
  (bind _returnvalue_2 (/ (+ (- (`self.StartX`) (`WidgetLayoutLibrary.GetMousePositionScaledByDPI` _returnvalue)) 1.0) -50.0))
  (if (`self.Enable`)
    (if (`self.Move`)
      (if (`PlayerController.IsInputKeyDown` _returnvalue "LeftMouseButton")
        (if (> (`KismetMathLibrary.Abs` _returnvalue_2) (`self.DeadZone`))
          (`SceneComponent.K2_AddRelativeRotation` (`self.Cube`) (`KismetMathLibrary.MakeRotator` 0.0 0.0 _returnvalue_2) false false)
          (bind _output_get (set `self.Direction` (> _returnvalue_2 0.0)))
          (if (!= (`self.LastDeadZone`) _output_get)
            (`self.CheckPass`))
          (set `self.LastDeadZone` _output_get)
          (`self.CheckPosition`))
        (else
          (set `self.Move` false))))))

(event `self.Cube.OnClicked`
  (params (TouchedComponent :type "PrimitiveComponent Object Reference") (ButtonPressed :type "Key Structure"))
  (bind (_locationx _locationy) (`WidgetLayoutLibrary.GetMousePositionScaledByDPI` (`GameplayStatics.GetPlayerController` 0)))
  (set `self.Move` true)
  (set `self.StartX` _locationx)
  (set `self.StartY` _locationy))

(event `Error`
  (`KismetSystemLibrary.K2_SetTimerDelegate` (delegate `ErrorEnd`) 0.2)
  (`PrimitiveComponent.SetMaterial` (`self.SM_SphereRed`) 0 "/Game/QuestKitMini/Materials/MI_EmissiveBase_R.MI_EmissiveBase_R"))

(event `ErrorEnd`
  (`PrimitiveComponent.SetMaterial` (`self.SM_SphereRed`) 0 null))

(fn `CheckPass`
  (bind _returnvalue (+ (`self.Progress`) 1))
  (if (`self.Valid`)
    (`self.UpdateProgress` _returnvalue)
    (if (== _returnvalue 6)
      (`self.onWin` self)
      (`self.Set View`)
      (set `self.Enable` false))
    (else
      (if (> (`self.Progress`) 0)
        (`self.Error`))
      (`self.UpdateProgress` 0)
      (`self.GeneratePass`))))

(fn `CheckPosition`
  (bind _output (`|GetArrayItem` (`self.Password`) (`self.Progress`)))
  (bind (_relativerotation_roll _relativerotation_pitch _relativerotation_yaw) (`KismetMathLibrary.BreakRotator` (`SceneComponent.RelativeRotation` (`self.Cube`))))
  (bind _returnvalue (`KismetMathLibrary.ClampAxis` _relativerotation_yaw))
  (bind _returnvalue_2 (and (> _returnvalue (`KismetMathLibrary.ClampAxis` (- _output (`self.ZoneSize`)))) (< _returnvalue (`KismetMathLibrary.ClampAxis` (+ _output (`self.ZoneSize`))))))
  (set `self.Valid` _returnvalue_2)
  (`self.SetStatus` (select `bool` _returnvalue_2 :`true` 1 :!type "Byte")))

(fn `GeneratePass`
  (`KismetArrayLibrary.Array_Clear` (`self.Password`))
  (for _ (range 7)
    (`KismetArrayLibrary.Array_Add` (`self.Password`) (`KismetMathLibrary.RandomFloatInRange` 3.0 357.0))))

(fn `SetStatus`
  (params (Index :type Byte))
  (`PrimitiveComponent.SetMaterial` (`self.SM_Sphere1`) 0 (select `byte` Index :`0` "/Game/QuestKitMini/Materials/MI_BaseB.MI_BaseB" :`1` "/Game/QuestKitMini/Materials/MI_EmissiveBase_G.MI_EmissiveBase_G" :!type "MaterialInterface Object Reference")))

(fn `UpdateProgress`
  (params (Progress :type Integer))
  (set `self.Progress` Progress)
  (for (_array_element _array_index) (`self.ProgressSM`)
    (`PrimitiveComponent.SetMaterial` _array_element 0 (select `bool` (> _array_index (- (`self.Progress`) 1)) :`false` "/Game/QuestKitMini/Materials/MI_GreenEmissive.MI_GreenEmissive" :`true` "/Game/QuestKitMini/Materials/MI_BaseB.MI_BaseB" :!type "MaterialInterface Object Reference"))))

(fn `UserConstructionScript`
  (set `self.ProgressSM` (`|MakeArray` (`self.SM_Progress01`) (`self.SM_Progress02`) (`self.SM_Progress03`) (`self.SM_Progress04`) (`self.SM_Progress05`))))