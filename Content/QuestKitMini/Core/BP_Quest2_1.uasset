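; BP_Quest2_1 is a quest-kit actor that displays two code sequences as rows of small textured meshes.
; Generate adds a static mesh per code element, spaced along Y from a start position, each with a dynamic material instance textured from TImages by that element's value.
; The construction script builds both rows from the default Code.
; GenerateCode destroys the existing meshes and rebuilds the rows from two supplied codes.
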(event `self.ReceiveBeginPlay`)

(fn `Generate`
  (params (Position :type "Vector Structure") (Code :type "Array of Integer"))
  (for (_array_element _array_index) Code
    (bind _returnvalue (`AddComponent|NODE_AddStaticMeshComponent-0` :`RelativeTransform` (`KismetMathLibrary.MakeTransform` (`KismetMathLibrary.MakeVector` (.x Position) (+ (.y Position) (`KismetMathLibrary.Conv_IntToDouble` (* _array_index -12))) (.z Position)) (struct :`Pitch` -90.0) (0.1 0.1 0.1))))
    (`KismetArrayLibrary.Array_Add` (`self.Meshes`) _returnvalue)
    (`SceneComponent.K2_AttachToComponent` _returnvalue (`self.DefaultSceneRoot`) "None" "KeepRelative" "KeepRelative" "KeepRelative" true)
    (bind _returnvalue_2 (`KismetMaterialLibrary.CreateDynamicMaterialInstance` "/Game/QuestKitMini/Materials/M_Button1_Mat.M_Button1_Mat"))
    (`MaterialInstanceDynamic.SetTextureParameterValue` _returnvalue_2 "Texture" (`|GetArrayItem` (`self.T_Images`) _array_element))
    (`PrimitiveComponent.SetMaterial` _returnvalue 0 _returnvalue_2)))

(fn `GenerateCode`
  (params (Code_1 :type "Array of Integer (by ref)") (Code_2 :type "Array of Integer (by ref)"))
  (for _array_element (`self.Meshes`)
    (`ActorComponent.K2_DestroyComponent` _array_element))
  (`KismetArrayLibrary.Array_Clear` (`self.Meshes`))
  (`self.Generate` (`self.StartPosition_1`) Code_1)
  (`self.Generate` (`self.StartPosition_2`) Code_2))

(fn `UserConstructionScript`
  (`self.Generate` (`self.StartPosition_1`) (`self.Code`))
  (`self.Generate` (`self.StartPosition_2`) (`self.Code`)))